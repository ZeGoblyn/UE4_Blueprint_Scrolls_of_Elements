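; BP_ExitZone is a kill-zone actor that deals damage over time to the first-person character while it overlaps the ExitZone component.
; Begin overlap casts to FirstPersonCharacter, stores it and starts a looping timer that applies 1 damage every second.
; End overlap by that stored character clears and invalidates the timer.
; BeginPlay initially sets the stored character to the player 0 pawn.
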(event `self.ReceiveTick`
  (params (DeltaSeconds :type "Float (single-precision)")))

(event `self.ReceiveActorBeginOverlap`
  (params (OtherActor :type "Actor Object Reference")))

(event `self.ReceiveBeginPlay`
  ;[0.08767 0.2135 0] Aquisition du personnage
  (set `self.Character` (`GameplayStatics.GetPlayerPawn` 0)))

(event `self.ExitZone.OnComponentBeginOverlap`
  (params (OverlappedComponent :type "PrimitiveComponent Object Reference") (OtherActor :type "Actor Object Reference") (OtherComp :type "PrimitiveComponent Object Reference") (OtherBodyIndex :type Integer) (bFromSweep :type Boolean) (SweepResult :type "HitResult Structure (by ref)"))
  ;[0.3219 0.00829 0] Gestion des dégats sur la durée
  (bind _asfirst_person_character (cast `/Game/Contenus/Acteurs/FirstPersonCharacter` OtherActor))
  (set `self.Character` _asfirst_person_character)
  (bind _returnvalue (`KismetSystemLibrary.K2_SetTimerDelegate` (delegate `Do damage`) 1.0 true))
  (set `self.Timer Handle` _returnvalue))

(event `Do damage`
  ;[0.3219 0.00829 0] Gestion des dégats sur la durée
  (`GameplayStatics.ApplyDamage` (`self.Character`) 1.0 null self))

(event `self.ExitZone.OnComponentEndOverlap`
  (params (OverlappedComponent :type "PrimitiveComponent Object Reference") (OtherActor :type "Actor Object Reference") (OtherComp :type "PrimitiveComponent Object Reference") (OtherBodyIndex :type Integer))
  ;[0.3219 0.00829 0] Gestion des dégats sur la durée
  (if (== OtherActor (`self.Character`))
    (`KismetSystemLibrary.K2_ClearAndInvalidateTimerHandle` (`self.Timer Handle`))))

(fn `UserConstructionScript`)